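; BP_CaptureTool sets up a camera capture tool that uses tagged actors as camera positions.
; BeginPlay sets the resolution, sorts CameraPosition-tagged actors by numeric display name, hands them and the camera to the child CameraController_Blueprint, then applies the first position.
; The S key toggles MainWidget on screen.
; Console-command chains for stereo panorama (SP) capture settings are present but never run.
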(event `self.ReceiveBeginPlay`
  (`|ExecutionSequence`
    (:`then_2`
      (`KismetSystemLibrary.ExecuteConsoleCommand` "r.setRes 1080x720" null))
    (:`then_3`
      ;[1 1 1] Initialize Position Array
      (bind _outactors (`GameplayStatics.GetAllActorsOfClassWithTag` "/Script/Engine.Actor" "CameraPosition"))
      (bind _ascamera_controller_blueprint (cast `/Game/Blueprints/InnerBlueprints/CameraController_Blueprint` (`ChildActorComponent.ChildActor` (`self.CameraController_Blueprint`))))
      (bind _output_get (set `self.Positions` _outactors))
      (`LowEntryExtendedStandardLibrary.SortObjectArrayDirectly` _output_get (`|CreateDelegate` :!event `Compare Name`))
      (set `/Game/Blueprints/InnerBlueprints/CameraController_Blueprint.PositionsAndRotations` _output_get _ascamera_controller_blueprint)
      (set `/Game/Blueprints/InnerBlueprints/CameraController_Blueprint.Camera` (`self.Camera`) _ascamera_controller_blueprint)
      (`/Game/Blueprints/InnerBlueprints/CameraController_Blueprint.SetPositionAndRo` _ascamera_controller_blueprint 0))))

(event `Key|S`
  (params (Key :type "Key Structure"))
  ;[1 1 1] Add and Remove Viewport
  (:`Pressed`
    (if (`self.UIOn`)
      (`Widget.RemoveFromParent` (stale _returnvalue))
      (set `self.UIOn` false)
      (else
        (bind _returnvalue (`|CreateWidget` "/Game/Blueprints/InnerBlueprints/mainWidget.mainWidget_C"))
        (`UserWidget.AddToViewport` _returnvalue 0)
        (set `self.UIOn` true)))))

(fn `Compare Name`
  (params (ObjectA :type "Object Object Reference") (ObjectB :type "Object Object Reference"))
  (returns (Result :type Boolean))
  (return (< (`KismetStringLibrary.Conv_StringToInt` (`KismetSystemLibrary.GetDisplayName` ObjectA)) (`KismetStringLibrary.Conv_StringToInt` (`KismetSystemLibrary.GetDisplayName` ObjectB)))))

(fn `UserConstructionScript`)
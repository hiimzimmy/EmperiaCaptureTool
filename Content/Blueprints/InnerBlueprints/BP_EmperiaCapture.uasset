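; Emperia capture Blueprint that takes 360-degree screenshots through Stereo Panoramic (SP.*) console commands.
; SingleCapture fires one panoramic screenshot.
; Capture does the same, waits a second, then calls CaptureFinished and prints a message about moving to the next frame.
; Console commands for movie capture, rendering, slice parameters, render passes, bit depth and mono mode are present but unwired, so they never run.
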(event `self.ReceiveBeginPlay`)

(event `SingleCapture`
  ;[1 1 1] Single Frame 360
  (`KismetSystemLibrary.ExecuteConsoleCommand` "SP.PanoramicScreenshot" null))

(event `Capture`
  ;[1 1 1] Single Frame 360
  (`KismetSystemLibrary.ExecuteConsoleCommand` "SP.PanoramicScreenshot" null)
  (`KismetSystemLibrary.Delay` 1.0)
  (`self.CaptureFinished`)
  (`KismetSystemLibrary.PrintString` "Capture Completed. Moving onto next frame in a second." true true (struct :`B` 0.011765 :`A` 1.0)))

(fn `UserConstructionScript`)
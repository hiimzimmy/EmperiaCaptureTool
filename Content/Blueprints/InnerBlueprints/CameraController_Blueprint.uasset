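; Camera controller that cycles a camera through preset viewpoints taken from an array of placed actors.
; Next and Previous events, also triggered by the Right and Left arrow keys, step an index with wraparound.
; Each step moves the camera to that actor's transform and sets the player controller's rotation to match.
; It also issues an SP.ForcedInitialYaw console command built from the viewpoint's yaw.
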(event `Next`
  ;[1 1 1] Next
  (if (> (+ (`self.CurrentInt`) 1) (- (`KismetArrayLibrary.Array_Length` (`self.PositionsAndRotations`)) 1)) :!label _label
    (set `self.CurrentInt` 0)
    (else
      (set `self.CurrentInt` (+ (`self.CurrentInt`) 1))))
  (`self.SetPositionAndRo` (`self.CurrentInt`)))

(event `Key|Right`
  (params (Key :type "Key Structure"))
  ;[1 1 1] Next
  (:`Pressed`
    (goto _label)))

(event `Key|Left`
  (params (Key :type "Key Structure"))
  ;[1 1 1] Previous
  (:`Pressed`
    (if (< (+ (`self.CurrentInt`) -1) 0) :!label _label_2
      (set `self.CurrentInt` (- (`KismetArrayLibrary.Array_Length` (`self.PositionsAndRotations`)) 1))
      (else
        (set `self.CurrentInt` (- (`self.CurrentInt`) 1))))
    (`self.SetPositionAndRo` (`self.CurrentInt`))))

(event `Previous`
  ;[1 1 1] Previous
  (goto _label_2))

(event `SetPositionAndRo`
  (params (int :type Integer))
  (bind (_returnvalue_location _returnvalue_rotation) (`KismetMathLibrary.BreakTransform` (`self.GetTransform` (`|GetArrayItem` (`self.PositionsAndRotations`) int))))
  ;[1 1 1] Camera Position And Rotation
  (`SceneComponent.K2_SetWorldLocationAndRotation` (`self.Camera`) _returnvalue_location _returnvalue_rotation false false)
  (`self.K2_SetActorRotation` (`GameplayStatics.GetPlayerController` 0) _returnvalue_rotation false)
  (`KismetSystemLibrary.ExecuteConsoleCommand` (`KismetStringLibrary.Concat_StrStr` "SP.ForcedInitialYaw " (`KismetStringLibrary.Conv_DoubleToString` (.yaw _returnvalue_rotation)) "f") null))

(fn `UserConstructionScript`)